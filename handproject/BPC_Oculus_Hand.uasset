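; Oculus hand component that detects finger curls and turns a point-then-thumb-press gesture into a teleport trigger.
; Each Tick, IsFIngerDown compares each fingertip or thumb-pad bone's distance to its socket against a threshold, updating per-finger flags.
; Pointing with middle, ring and pinky curled arms the gesture; lowering the thumb fires OnTeleport once until re-armed.
; The thumb check also draws debug points.
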(event EventBeginPlay)

(event EventTick
  (params (DeltaSeconds :type Float%20%28single-precision%29))
  (Utilities|FlowControl|Sequence
    (:then_0
      (bind _returnvalue (CallFunction|IsFIngerDown? (Variables|Default|GetThumbPad) (Variables|Default|GetThumbSocket) true 2.0))
      (if _returnvalue
        (if (not (Variables|Default|GetbThumbDown))
          (Variables|Default|SetbThumbDown (not (Variables|Default|GetbThumbDown)) :!label _label))
        (elif (Variables|Default|GetbThumbDown)
          (goto _label))))
    (:then_1
      (bind _returnvalue_2 (CallFunction|IsFIngerDown? (Variables|Default|GetIndexTip) (Variables|Default|GetIndexFingerSocket) false 1e+01))
      (if _returnvalue_2
        (if (not (Variables|Default|GetbIndexDown))
          (Variables|Default|SetbIndexDown (not (Variables|Default|GetbIndexDown)) :!label _label_2))
        (elif (Variables|Default|GetbIndexDown)
          (goto _label_2))))
    (:then_2
      (bind _returnvalue_3 (CallFunction|IsFIngerDown? (Variables|Default|GetMiddleTip) (Variables|Default|GetMiddleFingerSocket) false 4.0))
      (if _returnvalue_3
        (if (not (Variables|Default|GetbMiddleDown))
          (Variables|Default|SetbMiddleDown (not (Variables|Default|GetbMiddleDown)) :!label _label_3))
        (elif (Variables|Default|GetbMiddleDown)
          (goto _label_3))))
    (:then_3
      (bind _returnvalue_4 (CallFunction|IsFIngerDown? (Variables|Default|GetRingTip) (Variables|Default|GetRingFingerSocket) false 4.0))
      (if _returnvalue_4
        (if (not (Variables|Default|GetbRingDown))
          (Variables|Default|SetbRingDown (not (Variables|Default|GetbRingDown)) :!label _label_4))
        (elif (Variables|Default|GetbRingDown)
          (goto _label_4))))
    (:then_4
      (bind _returnvalue_5 (CallFunction|IsFIngerDown? (Variables|Default|GetPinkyTip) (Variables|Default|GetPinkyFingerSocket) false 4.0))
      (if _returnvalue_5
        (if (not (Variables|Default|GetbPinkyDown))
          (Variables|Default|SetbPinkyDown (not (Variables|Default|GetbPinkyDown)) :!label _label_5))
        (elif (Variables|Default|GetbPinkyDown)
          (goto _label_5))))
    (:then_5
      (if (Math|Boolean|ANDBoolean (Variables|Default|GetbMiddleDown) (Variables|Default|GetbRingDown) (Variables|Default|GetbPinkyDown) (not (Variables|Default|GetbIndexDown)) (not (Variables|Default|GetbThumbDown)))
        (Variables|Default|SetDisableTeleport false)
        (if (not (Variables|Default|GetbWasPointing?))
          (Variables|Default|SetbWasPointing? true))
        (elif (Math|Boolean|ANDBoolean (Variables|Default|GetbMiddleDown) (Variables|Default|GetbRingDown) (Variables|Default|GetbPinkyDown) (not (Variables|Default|GetbIndexDown)) (Variables|Default|GetbThumbDown))
          (if (Variables|Default|GetbWasPointing?)
            (if (not (Variables|Default|GetDisableTeleport))
              (Default|CallOnTeleport)
              (Variables|Default|SetDisableTeleport true)))
          (else
            (Variables|Default|SetbWasPointing? false)))))))

(fn IsFIngerDown?
  (params (BoneName :type Name) (SocketName :type Name) (Debug :type Boolean) (Threshold :type Float%20%28double-precision%29))
  (bind _returnvalue (Transformation|GetSocketLocation SocketName))
  (bind _returnvalue_2 (Class|PoseableMeshComponent|GetBoneLocationbyName BoneName "WorldSpace"))
  (if Debug
    (Rendering|Debug|DrawDebugPoint _returnvalue_2 2e+01 "(R=1.000000,G=0.001821,B=0.001821,A=1.000000)" 0.1)
    (Rendering|Debug|DrawDebugPoint _returnvalue 2e+01 "(R=0.056128,G=0.871367,B=0.068478,A=1.000000)" 0.1)
    (if (< (Math|Float|Absolute(Float) (Math|Vector|VectorLength (- _returnvalue_2 _returnvalue))) Threshold)
      (Rendering|Debug|DrawDebugPoint _returnvalue_2 21.0 "(R=0.871367,G=0.590619,B=0.054480,A=1.000000)" 0.1)
      (return (< (Math|Float|Absolute(Float) (Math|Vector|VectorLength (- _returnvalue_2 _returnvalue))) Threshold)))
    (else
      (return (< (Math|Float|Absolute(Float) (Math|Vector|VectorLength (- _returnvalue_2 _returnvalue))) Threshold)))))